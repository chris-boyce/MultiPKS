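; BP_DamageIndicator is a short-lived actor that displays a damage amount on a widget component.
; On BeginPlay it passes DamageAmount to its W_DamgeIndicator widget, stopping there if the cast fails.
; The MoveT timeline then lerps the actor from its spawn location to a fixed world-space offset, up and slightly sideways, and destroys it when finished.
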(event `self.ReceiveBeginPlay`
  (bind _asw_damge_indicator (cast `/Game/UI/W_DamgeIndicator` (`WidgetComponent.GetWidget` (`self.Widget`))))
  (set `/Game/UI/W_DamgeIndicator.DamageAmount` (`self.Damage Amount`) _asw_damge_indicator)
  (bind _output_get (set `self.StartLoc` (`self.K2_GetActorLocation`)))
  (set `self.EndLoc` (+ _output_get (-25.0 -25.0 50.0)))
  (bind (_direction _move_track) (`Timeline|Move T`)
    (:`Update`
      (`self.K2_SetActorLocation` (`KismetMathLibrary.VLerp` (`self.StartLoc`) (`self.EndLoc`) _move_track)))
    (:`Finished`
      (`self.K2_DestroyActor`))))

(fn `UserConstructionScript`)