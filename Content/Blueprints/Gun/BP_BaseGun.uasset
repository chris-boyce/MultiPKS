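; Base gun Blueprint that controls a Niagara glow particle effect reflecting the gun's value.
; EnableParticleSystem activates the glow and sets its linear color from TransformedGunValue through SetColorBasedOnValue, while DisableParticleSystem deactivates it.
; The construction script assigns the Sphere component to the SphereComponentZ variable.
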(event `self.EnableParticleSystem`
  (`ActorComponent.SetActive` (`self.NS_ParticleGlow`) true false)
  (bind _returnvalue (`UColorUtility.SetColorBasedOnValue` (`self.TransformedGunValue`)))
  (`NiagaraComponent.SetVariableLinearColor` (`self.NS_ParticleGlow`) "Linear Color" _returnvalue))

(event `self.DisableParticleSystem`
  (`ActorComponent.SetActive` (`self.NS_ParticleGlow`) false false))

(fn `UserConstructionScript`
  (set `self.SphereComponentZ` (`self.Sphere`)))