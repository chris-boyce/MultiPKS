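; Base enemy Blueprint that handles attacks, damage feedback and a loot drop.
; Attack requires a valid AI focus actor, then plays a placeholder sound and debug print and randomly starts either the laser or the projectile attack.
; DamageText spawns a damage indicator at the hit location and copies current health into the AI Blackboard.
; When destroyed, the enemy spawns a health pickup at its transform.
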(event `self.ReceiveDestroyed`
  (`|SpawnActorFromClass` "/Game/Models/BP_HealthPickup.BP_HealthPickup_C" (`self.GetTransform`) "Undefined" "MultiplyWithRoot" null null))

(event `self.DamageText`
  (params (Amount :type "Float (single-precision)") (HitLocation :type "Vector Structure"))
  (`|SpawnActorFromClass` "/Game/Blueprints/BP_DamageIndicator.BP_DamageIndicator_C" (`KismetMathLibrary.Conv_VectorToTransform` HitLocation) "Undefined" "MultiplyWithRoot" null Amount null)
  (`BlackboardComponent.SetValueAsFloat` (`AIBlueprintHelperLibrary.GetBlackboard` (`AIBlueprintHelperLibrary.GetAIController` self)) "Health" (`self.CurrentHealth`)))

(event `Attack`
  ;[1 0 0.007827] On the Tick See if Has Enemy in Focus
  (`/Engine/EditorBlueprintResources/StandardMacros.IsValid` (`AIController.GetFocusActor` (`AIBlueprintHelperLibrary.GetAIController` self))
    (:`Is Valid`
      ;[0 1 0.2538] Replace With New Attacks :-)
      (`GameplayStatics.PlaySoundAtLocation` "/Engine/VREditor/Sounds/UI/Click_on_Button_Cue.Click_on_Button_Cue" (`self.K2_GetActorLocation`) (struct) 1.0 1.0 0.0 null null null null)
      (`KismetSystemLibrary.PrintString` "Firing")
      (if (`KismetMathLibrary.RandomBool`)
        (`EnemyAttackLaser.BeginAttack` (`self.BP_EnemyAttackLaser`))
        (else
          (`EnemyAttackProjectile.BeginAttack` (`self.BP_EnemyAttackProjectile`)))))))

(fn `UserConstructionScript`)