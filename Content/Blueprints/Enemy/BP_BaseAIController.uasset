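; BP_BaseAIController is the base enemy AI controller, running the BT_BaseAI behavior tree on begin play.
; When AI perception senses a BP_ThirdPersonCharacter, it writes it to the TargetActor blackboard key, focuses on it and cancels any pending lose-target timer.
; When sensing fails, a short grace-period timer starts, then clears the blackboard target and focus.
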(event `self.ReceiveBeginPlay`
  (`self.RunBehaviorTree` "/Game/Blueprints/Enemy/BT_BaseAI.BT_BaseAI"))

(event `self.AIPerception.OnTargetPerceptionUpdated`
  (params (Actor :type "Actor Object Reference") (Stimulus :type "AIStimulus Structure"))
  (bind _output_get (set `self.Actor` Actor))
  (cast `/Game/Blueprints/Player/BP_ThirdPersonCharacter` _output_get)
  (if (`.bSuccessfullySensed` (break `AIStimulus` Stimulus))
    (`BlackboardComponent.SetValueAsObject` (`self.Blackboard`) "TargetActor" (`self.Actor`))
    (`self.K2_SetFocus` (`self.Actor`))
    (`KismetSystemLibrary.K2_ClearAndInvalidateTimerHandle` (`self.LoseTargetTimer`))
    (else
      (bind _returnvalue (`KismetSystemLibrary.K2_SetTimerDelegate` (delegate `LooseTarget`) 3.0))
      (set `self.LoseTargetTimer` _returnvalue))))

(event `LooseTarget`
  (`BlackboardComponent.SetValueAsObject` (`self.Blackboard`) "TargetActor" null)
  (`self.K2_ClearFocus`))

(fn `UserConstructionScript`)