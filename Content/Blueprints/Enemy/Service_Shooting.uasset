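; Behavior tree service for enemy AI that triggers an attack when the controller's focus actor is in clear view.
; On activation it caches the controlled BP_BaseEnemy and its controller.
; Each tick it sphere-traces on the Camera channel from the pawn to the focus actor, ignoring itself, and calls Attack only if that actor is the first hit.
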(event `self.ReceiveActivationAI`
  (params (OwnerController :type "AIController Object Reference") (ControlledPawn :type "Pawn Object Reference"))
  (bind _asbp_base_enemy (cast `/Game/Blueprints/Enemy/BP_BaseEnemy` ControlledPawn))
  (set `self.As BP Base Enemy` _asbp_base_enemy)
  (set `self.Owner Controller` OwnerController))

(event `self.ReceiveTickAI`
  (params (OwnerController :type "AIController Object Reference") (ControlledPawn :type "Pawn Object Reference") (DeltaSeconds :type "Float (single-precision)"))
  (bind (_outhit _returnvalue) (`KismetSystemLibrary.SphereTraceSingle` (`Actor.K2_GetActorLocation` ControlledPawn) (`Actor.K2_GetActorLocation` (`AIController.GetFocusActor` OwnerController)) 64.0 "TraceTypeQuery2" false (`|MakeArray` (`self.As BP Base Enemy`) :!type "Actor Object Reference")))
  (if _returnvalue
    (if (== (`.HitActor` (`GameplayStatics.BreakHitResult` _outhit)) (`AIController.GetFocusActor` (`self.Owner Controller`)))
      (`/Game/Blueprints/Enemy/BP_BaseEnemy.Attack` (`self.As BP Base Enemy`)))))