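; BP_BaseGun is a gun base Blueprint built from barrel, scope and magazine components.
; EnableOutline and DisableOutline toggle custom depth rendering on the static meshes of those three parts to switch the gun's outline on and off.
; The construction script assigns the Sphere component to the SphereComponentZ variable.
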(event `self.EnableOutline`
  (`PrimitiveComponent.SetRenderCustomDepth` (`Barrel.StaticMeshComponent` (`self.BarrelComponent`)) true)
  (`PrimitiveComponent.SetRenderCustomDepth` (`Scope.StaticMeshComponent` (`self.ScopeComponent`)) true)
  (`PrimitiveComponent.SetRenderCustomDepth` (`Magazine.StaticMeshComponent` (`self.MagazineComponent`)) true))

(event `self.DisableOutline`
  (`PrimitiveComponent.SetRenderCustomDepth` (`Barrel.StaticMeshComponent` (`self.BarrelComponent`)) false)
  (`PrimitiveComponent.SetRenderCustomDepth` (`Scope.StaticMeshComponent` (`self.ScopeComponent`)) false)
  (`PrimitiveComponent.SetRenderCustomDepth` (`Magazine.StaticMeshComponent` (`self.MagazineComponent`)) false))

(fn `UserConstructionScript`
  (set `self.SphereComponentZ` (`self.Sphere`)))