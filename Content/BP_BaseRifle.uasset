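; BP_BaseRifle is a base rifle actor assembled from separate mesh parts such as aim, back, bottom, handle, middle, muzzle and top.
; Its EnableOutline event turns on custom depth rendering for those parts for two seconds, then turns it off, providing a timed highlight.
; The construction script assigns its Sphere component to the SphereComponentZ variable.
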(event `self.EnableOutline`
  (`PrimitiveComponent.SetRenderCustomDepth` (`self.Aim_01`) true)
  (`PrimitiveComponent.SetRenderCustomDepth` (`self.Back_Part_01`) true)
  (`PrimitiveComponent.SetRenderCustomDepth` (`self.Bottom_Part_01`) true)
  (`PrimitiveComponent.SetRenderCustomDepth` (`self.Handle_01`) true)
  (`PrimitiveComponent.SetRenderCustomDepth` (`self.Middle_Part_01`) true)
  (`PrimitiveComponent.SetRenderCustomDepth` (`self.Muzzle_04`) true)
  (`PrimitiveComponent.SetRenderCustomDepth` (`self.Top_Part_01`) true)
  (`KismetSystemLibrary.Delay` 2.0)
  (`PrimitiveComponent.SetRenderCustomDepth` (`self.Aim_01`) false)
  (`PrimitiveComponent.SetRenderCustomDepth` (`self.Back_Part_01`) false)
  (`PrimitiveComponent.SetRenderCustomDepth` (`self.Bottom_Part_01`) false)
  (`PrimitiveComponent.SetRenderCustomDepth` (`self.Handle_01`) false)
  (`PrimitiveComponent.SetRenderCustomDepth` (`self.Middle_Part_01`) false)
  (`PrimitiveComponent.SetRenderCustomDepth` (`self.Muzzle_04`) false)
  (`PrimitiveComponent.SetRenderCustomDepth` (`self.Top_Part_01`) false))

(fn `UserConstructionScript`
  (set `self.SphereComponentZ` (`self.Sphere`)))