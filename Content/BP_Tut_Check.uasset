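; Tutorial check actor that removes its own Cube component once two referenced actors have been destroyed.
; On BeginPlay it binds one shared handler to the OnDestroyed events of A1 and A2.
; Each call increments a counter, and the Cube component is destroyed when the count reaches two.
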(event `self.ReceiveBeginPlay`
  (add `self.OnDestroyed` (`self.A1`) (delegate `OnDestroyed_Event`))
  (add `self.OnDestroyed` (`self.A2`) (delegate `OnDestroyed_Event`)))

(event `OnDestroyed_Event` :!signature `self.OnDestroyed`
  (params (DestroyedActor :type "Actor Object Reference"))
  (bind _result (`/Engine/EditorBlueprintResources/StandardMacros.IncrementInt` (`self.Count`))
    (:`  `
      (set `self.Count` _result)
      (if (== (`self.Count`) 2)
        (`ActorComponent.K2_DestroyComponent` (`self.Cube`))))))

(fn `UserConstructionScript`)