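; Tutorial end pressure plate that moves the session to ThirdPersonMap when two actors stand on it at once.
; Begin and end overlap events raise and lower PlayerCount, with no check on what kind of actor overlaps.
; When the count reaches exactly two, it calls ServerTravel and prints the returned result.
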(event `self.ReceiveActorBeginOverlap`
  (params (OtherActor :type "Actor Object Reference"))
  (bind _result (`/Engine/EditorBlueprintResources/StandardMacros.IncrementInt` (`self.PlayerCount`))
    (:`  `
      (bind _output_get (set `self.PlayerCount` _result))
      (if (== _output_get 2)
        (bind _returnvalue (`AdvancedSessionsLibrary.ServerTravel` "ThirdPersonMap"))
        (`KismetSystemLibrary.PrintString` (`KismetStringLibrary.Conv_BoolToString` _returnvalue))))))

(event `self.ReceiveActorEndOverlap`
  (params (OtherActor :type "Actor Object Reference"))
  (bind _result (`/Engine/EditorBlueprintResources/StandardMacros.DecrementInt` (`self.PlayerCount`))
    (:`  `
      (set `self.PlayerCount` _result))))

(fn `UserConstructionScript`)